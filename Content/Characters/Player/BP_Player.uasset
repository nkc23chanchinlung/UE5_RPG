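; BP_Player is the player character Blueprint, translating input into movement, camera look, jumping and an attack request.
; Movement axes follow control-rotation yaw only, so camera pitch does not affect direction, while look axes drive controller yaw and pitch.
; The jump action calls Jump, and the attack action only sets an Attack flag, which nothing in this graph reads or resets.
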(event `InputAction|Attack1`
  (params (Key :type "Key Structure"))
  (:`Pressed`
    (set `self.Attack` true)))

(event `InputAction|MyJump`
  (params (Key :type "Key Structure"))
  (:`Pressed`
    (`self.Jump`)))

(event `InputAxis|MoveForward/Back`
  (params (AxisValue :type "Float (single-precision)"))
  (bind (_returnvalue_roll _returnvalue_pitch _returnvalue_yaw) (`KismetMathLibrary.BreakRotator` (`self.GetControlRotation`)))
  ; 移動処理
  (`self.AddMovementInput` (`KismetMathLibrary.GetForwardVector` (`KismetMathLibrary.MakeRotator` 0.0 0.0 _returnvalue_yaw)) AxisValue))

(event `InputAxis|MoveLeft/Right`
  (params (AxisValue :type "Float (single-precision)"))
  (bind (_returnvalue_roll _returnvalue_pitch _returnvalue_yaw) (`KismetMathLibrary.BreakRotator` (`self.GetControlRotation`)))
  ; 移動処理
  (`self.AddMovementInput` (`KismetMathLibrary.GetRightVector` (`KismetMathLibrary.MakeRotator` 0.0 0.0 _returnvalue_yaw)) AxisValue))

(event `InputAxis|LookLeft/Right`
  (params (AxisValue :type "Float (single-precision)"))
  ; カメラ移動
  (`self.AddControllerYawInput` AxisValue))

(event `InputAxis|LookUP/Down`
  (params (AxisValue :type "Float (single-precision)"))
  ; カメラ移動
  (`self.AddControllerPitchInput` AxisValue))

(fn `UserConstructionScript`)